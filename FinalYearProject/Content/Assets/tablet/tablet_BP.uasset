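; VR tablet that lets the player raise, lower and rotate the LiftBP's Cylinder with fingertip buttons.
; Overlaps from a pointing BP_MotionController's FingerCollider set Up, Down or Rotate flags, cleared when the finger leaves.
; While the tablet is visible, Tick applies one fixed, frame-rate-dependent step by priority (up, down, rotate), with height limits.
; A left controller face button toggles visibility, which Tick reapplies to the meshes every frame.
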(event `self.ReceiveTick`
  (params (DeltaSeconds :type "Float (single-precision)"))
  (`self.moveLift`)
  (`self.Hide Tablet`))

(event `self.ReceiveBeginPlay`
  (bind _outactors (`GameplayStatics.GetAllActorsOfClass` "/Game/Assets/room/lift/liftBP.liftBP_C"))
  (for _array_element _outactors
    (set `self.lift` _array_element)))

(event `self.upButton.OnComponentBeginOverlap`
  (params (OverlappedComponent :type "PrimitiveComponent Object Reference") (OtherActor :type "Actor Object Reference") (OtherComp :type "PrimitiveComponent Object Reference") (OtherBodyIndex :type Integer) (bFromSweep :type Boolean) (SweepResult :type "HitResult Structure (by ref)"))
  ;[1 1 1] up/down/rotate button collison check
  (bind _asbp_motion_controller (cast `/Game/VirtualRealityBP/Blueprints/BP_MotionController` OtherActor))
  (if (`/Game/VirtualRealityBP/Blueprints/BP_MotionController.isPointing` _asbp_motion_controller)
    (if (== OtherComp (`/Game/VirtualRealityBP/Blueprints/BP_MotionController.fingerCollider` _asbp_motion_controller))
      (set `self.isUp` true))))

(event `moveLift`
  (bind _cylinder (`/Game/Assets/room/lift/liftBP.Cylinder` (`self.lift`)))
  (bind (_returnvalue_x _returnvalue_y _returnvalue_z) (`KismetMathLibrary.BreakVector` (`SceneComponent.K2_GetComponentLocation` _cylinder)))
  (if (`self.isVisable`)
    (if (`self.isUp`)
      (if (< _returnvalue_z 83.57)
        (`SceneComponent.K2_AddLocalOffset` _cylinder (0.0 0.0 1.0) false false))
      (elif (`self.isDown`)
        (if (> _returnvalue_z -230.0)
          (`SceneComponent.K2_AddLocalOffset` _cylinder (0.0 0.0 -1.0) false false))
        (elif (`self.isRotate`)
          (`SceneComponent.K2_AddWorldRotation` _cylinder (struct :`Yaw` 1.0) false false))))))

(event `self.upButton.OnComponentEndOverlap`
  (params (OverlappedComponent :type "PrimitiveComponent Object Reference") (OtherActor :type "Actor Object Reference") (OtherComp :type "PrimitiveComponent Object Reference") (OtherBodyIndex :type Integer))
  ;[1 1 1] up/down/rotate button collison check
  (bind _asbp_motion_controller (cast `/Game/VirtualRealityBP/Blueprints/BP_MotionController` OtherActor))
  (if (== OtherComp (`/Game/VirtualRealityBP/Blueprints/BP_MotionController.fingerCollider` _asbp_motion_controller))
    (set `self.isUp` false)))

(event `self.downButton.OnComponentBeginOverlap`
  (params (OverlappedComponent :type "PrimitiveComponent Object Reference") (OtherActor :type "Actor Object Reference") (OtherComp :type "PrimitiveComponent Object Reference") (OtherBodyIndex :type Integer) (bFromSweep :type Boolean) (SweepResult :type "HitResult Structure (by ref)"))
  ;[1 1 1] up/down/rotate button collison check
  (bind _asbp_motion_controller (cast `/Game/VirtualRealityBP/Blueprints/BP_MotionController` OtherActor))
  (if (`/Game/VirtualRealityBP/Blueprints/BP_MotionController.isPointing` _asbp_motion_controller)
    (if (== OtherComp (`/Game/VirtualRealityBP/Blueprints/BP_MotionController.fingerCollider` _asbp_motion_controller))
      (set `self.isDown` true))))

(event `self.downButton.OnComponentEndOverlap`
  (params (OverlappedComponent :type "PrimitiveComponent Object Reference") (OtherActor :type "Actor Object Reference") (OtherComp :type "PrimitiveComponent Object Reference") (OtherBodyIndex :type Integer))
  ;[1 1 1] up/down/rotate button collison check
  (bind _asbp_motion_controller (cast `/Game/VirtualRealityBP/Blueprints/BP_MotionController` OtherActor))
  (if (== OtherComp (`/Game/VirtualRealityBP/Blueprints/BP_MotionController.fingerCollider` _asbp_motion_controller))
    (set `self.isDown` false)))

(event `self.rotateButton.OnComponentBeginOverlap`
  (params (OverlappedComponent :type "PrimitiveComponent Object Reference") (OtherActor :type "Actor Object Reference") (OtherComp :type "PrimitiveComponent Object Reference") (OtherBodyIndex :type Integer) (bFromSweep :type Boolean) (SweepResult :type "HitResult Structure (by ref)"))
  ;[1 1 1] up/down/rotate button collison check
  (bind _asbp_motion_controller (cast `/Game/VirtualRealityBP/Blueprints/BP_MotionController` OtherActor))
  (if (`/Game/VirtualRealityBP/Blueprints/BP_MotionController.isPointing` _asbp_motion_controller)
    (if (== OtherComp (`/Game/VirtualRealityBP/Blueprints/BP_MotionController.fingerCollider` _asbp_motion_controller))
      (set `self.isRotate` true))))

(event `self.rotateButton.OnComponentEndOverlap`
  (params (OverlappedComponent :type "PrimitiveComponent Object Reference") (OtherActor :type "Actor Object Reference") (OtherComp :type "PrimitiveComponent Object Reference") (OtherBodyIndex :type Integer))
  ;[1 1 1] up/down/rotate button collison check
  (bind _asbp_motion_controller (cast `/Game/VirtualRealityBP/Blueprints/BP_MotionController` OtherActor))
  (if (== OtherComp (`/Game/VirtualRealityBP/Blueprints/BP_MotionController.fingerCollider` _asbp_motion_controller))
    (set `self.isRotate` false)))

(event `Key|MotionController_Left_FaceButton2`
  (params (Key :type "Key Structure"))
  (:`Pressed`
    (set `self.isVisable` (not (`self.isVisable`)))))

(event `Hide Tablet`
  (`SceneComponent.SetVisibility` (`self.Cube`) (`self.isVisable`) false)
  (`SceneComponent.SetVisibility` (`self.downButton`) (`self.isVisable`) false)
  (`SceneComponent.SetVisibility` (`self.rotateButton`) (`self.isVisable`) false)
  (`SceneComponent.SetVisibility` (`self.upButton`) (`self.isVisable`) false))

(fn `UserConstructionScript`)